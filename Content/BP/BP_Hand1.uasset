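; VR hand actor for Oculus hand tracking that can click UI widgets through a WidgetInteraction component.
; The construction script sets the motion source and Oculus hand mesh and skeleton from the Hand side.
; BeginPlay assigns a virtual user per side, and Press and Release drive a virtual left mouse button.
; Pointer-pose aiming and spline laser logic, gated on tracking confidence, is present but unconnected, so it never runs.
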(event `self.ReceiveBeginPlay`
  (bind _widgetinteraction (`self.WidgetInteraction`))
  (switch `EControllerHand` (`self.Hand`)
    (:`Left`
      (set `WidgetInteractionComponent.VirtualUserIndex` 0 _widgetinteraction))
    (:`Right`
      (set `WidgetInteractionComponent.VirtualUserIndex` 1 _widgetinteraction))))

(event `Press`
  (`WidgetInteractionComponent.PressPointerKey` (`self.WidgetInteraction`) "LeftMouseButton"))

(event `Release`
  (`WidgetInteractionComponent.ReleasePointerKey` (`self.WidgetInteraction`) "LeftMouseButton"))

(event `self.ReceiveTick`
  (params (DeltaSeconds :type "Float (single-precision)")))

(fn `Get Oculus Hand`
  (returns (ReturnValue :type "EOculusXRHandType Enum"))
  (return (select `EControllerHand` (`self.Hand`) :`Left` "HandLeft" :`Right` "HandRight" :!type "EOculusXRHandType Enum")))

(fn `UserConstructionScript`
  (bind _returnvalue (`self.Get Oculus Hand`))
  (bind _oculusxrhand (`self.OculusXRHand`))
  (set `MotionControllerComponent.MotionSource` (`|GetEnumeratorName` (`self.Hand`)) (`self.MotionController`))
  (set `OculusXRHandComponent.MeshType` _returnvalue _oculusxrhand)
  (set `OculusXRHandComponent.SkeletonType` _returnvalue _oculusxrhand))