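; BP_Hand is a per-side Oculus hand-tracking actor that points at and clicks widgets with a laser.
; Construction configures the motion controller and hand mesh from the Hand enum; BeginPlay gives each side its own virtual user index.
; On high tracking confidence, Tick aligns WidgetInteraction and spline to the pointer pose, stretching the beam to hits or collapsing it otherwise.
; Very short beams set IsClicked; Press and Release send left-mouse clicks.
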(event `self.ReceiveBeginPlay`
  (bind _widgetinteraction (`self.WidgetInteraction`))
  (switch `EControllerHand` (`self.Hand`)
    (:`Left`
      (set `WidgetInteractionComponent.VirtualUserIndex` 0 _widgetinteraction))
    (:`Right`
      (set `WidgetInteractionComponent.VirtualUserIndex` 1 _widgetinteraction))))

(event `Press`
  (`WidgetInteractionComponent.PressPointerKey` (`self.WidgetInteraction`) "LeftMouseButton"))

(event `Release`
  (`WidgetInteractionComponent.ReleasePointerKey` (`self.WidgetInteraction`) "LeftMouseButton"))

(event `self.ReceiveTick`
  (params (DeltaSeconds :type "Float (single-precision)"))
  (bind _returnvalue (`self.GetTransform`))
  (bind _splinemesh (`self.SplineMesh`))
  (bind (_returnvalue_location _returnvalue_rotation) (`KismetMathLibrary.BreakTransform` (`OculusXRInputFunctionLibrary.GetPointerPose` (`self.Get Oculus Hand`))))
  (bind (_bblockinghit _binitialoverlap _time _distance _location) (`GameplayStatics.BreakHitResult` (`WidgetInteractionComponent.GetLastHitResult` (`self.WidgetInteraction`))))
  (switch `EOculusXRTrackingConfidence` (`OculusXRInputFunctionLibrary.GetTrackingConfidence` (`self.Get Oculus Hand`))
    (:`Low`
      (`self.CollapseSpline`))
    (:`High`
      (if (`OculusXRInputFunctionLibrary.IsPointerPoseValid` (`self.Get Oculus Hand`))
        (`SceneComponent.K2_SetWorldLocationAndRotation` (`self.WidgetInteraction`) (`KismetMathLibrary.TransformLocation` _returnvalue _returnvalue_location) (`KismetMathLibrary.TransformRotation` _returnvalue _returnvalue_rotation) false false)
        (`SceneComponent.K2_SetWorldLocationAndRotation` (`self.Spline`) (`KismetMathLibrary.TransformLocation` _returnvalue _returnvalue_location) (`KismetMathLibrary.TransformRotation` _returnvalue _returnvalue_rotation) false false)
        (if _bblockinghit
          (`SplineComponent.SetLocationAtSplinePoint` (`self.Spline`) 1 _location "World" true)
          (`self.UpdateSplineMesh`)
          (if (< (`KismetMathLibrary.Vector_Distance` (`SplineMeshComponent.GetStartPosition` _splinemesh) (`SplineMeshComponent.GetEndPosition` _splinemesh)) 4.0)
            (set `self.IsClicked` true)
            (else
              (set `self.IsClicked` false)))
          (else
            (`self.CollapseSpline`)))
        (else
          (`self.CollapseSpline`))))))

(fn `CollapseSpline`
  (`SplineComponent.SetLocationAtSplinePoint` (`self.Spline`) 1 (`SplineComponent.GetLocationAtSplinePoint` (`self.Spline`) 0 "World") "World" true)
  (`self.UpdateSplineMesh`))

(fn `Get Oculus Hand`
  (returns (ReturnValue :type "EOculusXRHandType Enum"))
  (return (select `EControllerHand` (`self.Hand`) :`Left` "HandLeft" :`Right` "HandRight" :!type "EOculusXRHandType Enum")))

(fn `UpdateSplineMesh`
  (bind _spline (`self.Spline`))
  (bind (_location _tangent) (`SplineComponent.GetLocationAndTangentAtSplinePoint` _spline 1 "Local"))
  (bind (_location_2 _tangent_2) (`SplineComponent.GetLocationAndTangentAtSplinePoint` _spline 0 "Local"))
  (`SplineMeshComponent.SetStartAndEnd` (`self.SplineMesh`) _location_2 _tangent_2 _location _tangent true))

(fn `UserConstructionScript`
  (bind _returnvalue (`self.Get Oculus Hand`))
  (bind _oculusxrhand (`self.OculusXRHand`))
  (set `MotionControllerComponent.MotionSource` (`|GetEnumeratorName` (`self.Hand`)) (`self.MotionController`))
  (set `OculusXRHandComponent.MeshType` _returnvalue _oculusxrhand)
  (set `OculusXRHandComponent.SkeletonType` _returnvalue _oculusxrhand))