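; BP_Menutake is a subway kiosk menu screen actor that hosts the Kiosk_take widget and switches to another screen after a selection.
; Tick polls the widget's Selected flag, then uses Next to choose between BP_MenuSand and the fallback BP_MainMenu.
; After a short delay it destroys itself and spawns that screen actor at its own transform.
; Leftover Kiosk_sand and sound nodes are unconnected.
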(event `self.ReceiveBeginPlay`)

(event `self.ReceiveTick`
  (params (DeltaSeconds :type "Float (single-precision)"))
  (bind _returnvalue (`WidgetComponent.GetWidget` (`self.Widget`)))
  (bind _askiosk_take (cast `/Game/BP/SubwayWidget2/Kiosk_take` _returnvalue))
  (if (`/Game/BP/SubwayWidget2/Kiosk_take.Selected` _askiosk_take)
    (bind _askiosk_take_2 (cast `/Game/BP/SubwayWidget2/Kiosk_take` _returnvalue))
    (if (`/Game/BP/SubwayWidget2/Kiosk_take.Next` _askiosk_take_2)
      (`KismetSystemLibrary.Delay` 1.0)
      (`self.K2_DestroyActor`)
      (`|SpawnActorFromClass` "/Game/BP/SubwayWidget2/BP_MenuSand.BP_MenuSand_C" (`self.GetTransform`) "Undefined" "MultiplyWithRoot" null null)
      (else
        (`KismetSystemLibrary.Delay` 1.0)
        (`self.K2_DestroyActor`)
        (`|SpawnActorFromClass` "/Game/BP/SubwayWidget2/BP_MainMenu.BP_MainMenu_C" (`self.GetTransform`) "Undefined" "MultiplyWithRoot" null null)))))

(fn `UserConstructionScript`)