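; BP_MenuPayFinish is an actor that hosts the payment-finish screen of a kiosk menu through its Widget component.
; Tick casts the hosted widget to Kiosk_payFinish and polls its Reset flag.
; When the flag is set, the actor destroys itself and spawns BP_MainMenu at its own transform, returning the kiosk to the main menu.
; A disconnected leftover that reads Eggmayovec from Kiosk_sand never runs.
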(event `self.ReceiveBeginPlay`)

(event `self.ReceiveTick`
  (params (DeltaSeconds :type "Float (single-precision)"))
  (bind _askiosk_pay_finish (cast `/Game/BP/SubwayWidget2/Kiosk_payFinish` (`WidgetComponent.GetWidget` (`self.Widget`))))
  (if (`/Game/BP/SubwayWidget2/Kiosk_payFinish.reset` _askiosk_pay_finish)
    (`self.K2_DestroyActor`)
    (`|SpawnActorFromClass` "/Game/BP/SubwayWidget2/BP_MainMenu.BP_MainMenu_C" (`self.GetTransform`) "Undefined" "MultiplyWithRoot" null null)))

(fn `UserConstructionScript`)