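; BP_MenuPayNaver is the kiosk menu actor for the Naver Pay screen, hosting a Kiosk_payNaver widget.
; Every Tick it polls the widget's Pre and Pay flags, with Pre checked first.
; Pre swaps it for BP_MenuSelectPay and Pay for BP_MenuPayFinish, by destroying itself and spawning the next actor at its transform.
; An unconnected Kiosk_sand cast that reads Eggmayovec never runs.
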(event `self.ReceiveBeginPlay`)

(event `self.ReceiveTick`
  (params (DeltaSeconds :type "Float (single-precision)"))
  (bind _returnvalue (`WidgetComponent.GetWidget` (`self.Widget`)))
  (bind _askiosk_pay_naver (cast `/Game/BP/SubwayWidget2/Kiosk_payNaver` _returnvalue))
  (if (`/Game/BP/SubwayWidget2/Kiosk_payNaver.Pre` _askiosk_pay_naver)
    (`self.K2_DestroyActor`)
    (`|SpawnActorFromClass` "/Game/BP/SubwayWidget2/BP_MenuSelectPay.BP_MenuSelectPay_C" (`self.GetTransform`) "Undefined" "MultiplyWithRoot" null null)
    (else
      (bind _askiosk_pay_naver_2 (cast `/Game/BP/SubwayWidget2/Kiosk_payNaver` _returnvalue))
      (if (`/Game/BP/SubwayWidget2/Kiosk_payNaver.Pay` _askiosk_pay_naver_2)
        (`self.K2_DestroyActor`)
        (`|SpawnActorFromClass` "/Game/BP/SubwayWidget2/BP_MenuPayFinish.BP_MenuPayFinish_C" (`self.GetTransform`) "Undefined" "MultiplyWithRoot" null null)))))

(fn `UserConstructionScript`)