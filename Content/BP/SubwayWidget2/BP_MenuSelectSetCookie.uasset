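; BP_MenuSelectSetCookie is the cookie selection screen actor in a kiosk's set menu flow, hosting a Kiosk_SelectCookie widget.
; Tick polls the widget's flags and acts once Selected is true.
; Next with Cookie set advances to BP_MenuSelectSetDrink, while Next unset returns to BP_MenuSelectSet.
; Screens switch by destroying this actor and spawning the replacement at the same transform.
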(event `self.ReceiveBeginPlay`)

(event `self.ReceiveTick`
  (params (DeltaSeconds :type "Float (single-precision)"))
  (bind _returnvalue (`WidgetComponent.GetWidget` (`self.Widget`)))
  (bind _askiosk_select_cookie (cast `/Game/BP/SubwayWidget2/Kiosk_SelectCookie` _returnvalue))
  (if (`/Game/BP/SubwayWidget2/Kiosk_SelectCookie.Selected` _askiosk_select_cookie)
    (bind _askiosk_select_cookie_2 (cast `/Game/BP/SubwayWidget2/Kiosk_SelectCookie` _returnvalue))
    (if (`/Game/BP/SubwayWidget2/Kiosk_SelectCookie.Next` _askiosk_select_cookie_2)
      (bind _askiosk_select_cookie_3 (cast `/Game/BP/SubwayWidget2/Kiosk_SelectCookie` _returnvalue))
      (if (`/Game/BP/SubwayWidget2/Kiosk_SelectCookie.Cookie` _askiosk_select_cookie_3)
        (`self.K2_DestroyActor`)
        (`|SpawnActorFromClass` "/Game/BP/SubwayWidget2/BP_MenuSelectSetDrink.BP_MenuSelectSetDrink_C" (`self.GetTransform`) "Undefined" "MultiplyWithRoot" null null))
      (else
        (`self.K2_DestroyActor`)
        (`|SpawnActorFromClass` "/Game/BP/SubwayWidget2/BP_MenuSelectSet.BP_MenuSelectSet_C" (`self.GetTransform`) "Undefined" "MultiplyWithRoot" null null)))))

(fn `UserConstructionScript`)