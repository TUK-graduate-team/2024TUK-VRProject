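; BP_MenuSelectSetDrink is an actor for the drink-selection screen in a kiosk ordering flow.
; Every Tick it polls its Kiosk_SelectDrink widget's flags rather than reacting to events.
; Once Selected is set, it swaps itself for the next screen actor at the same transform.
; Next plus Drink spawns BP_MenuSelectPay, while Selected without Next spawns BP_MenuSelectSetCookie.
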(event `self.ReceiveBeginPlay`)

(event `self.ReceiveTick`
  (params (DeltaSeconds :type "Float (single-precision)"))
  (bind _returnvalue (`WidgetComponent.GetWidget` (`self.Widget`)))
  (bind _askiosk_select_drink (cast `/Game/BP/SubwayWidget2/Kiosk_SelectDrink` _returnvalue))
  (if (`/Game/BP/SubwayWidget2/Kiosk_SelectDrink.Selected` _askiosk_select_drink)
    (bind _askiosk_select_drink_2 (cast `/Game/BP/SubwayWidget2/Kiosk_SelectDrink` _returnvalue))
    (if (`/Game/BP/SubwayWidget2/Kiosk_SelectDrink.Next` _askiosk_select_drink_2)
      (bind _askiosk_select_drink_3 (cast `/Game/BP/SubwayWidget2/Kiosk_SelectDrink` _returnvalue))
      (if (`/Game/BP/SubwayWidget2/Kiosk_SelectDrink.Drink` _askiosk_select_drink_3)
        (`self.K2_DestroyActor`)
        (`|SpawnActorFromClass` "/Game/BP/SubwayWidget2/BP_MenuSelectPay.BP_MenuSelectPay_C" (`self.GetTransform`) "Undefined" "MultiplyWithRoot" null null))
      (else
        (`self.K2_DestroyActor`)
        (`|SpawnActorFromClass` "/Game/BP/SubwayWidget2/BP_MenuSelectSetCookie.BP_MenuSelectSetCookie_C" (`self.GetTransform`) "Undefined" "MultiplyWithRoot" null null)))))

(fn `UserConstructionScript`)