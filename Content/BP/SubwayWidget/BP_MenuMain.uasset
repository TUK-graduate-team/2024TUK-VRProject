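; BP_MenuMain is a main-menu actor for the subway kiosk that hosts a Kiosk_Main widget through a widget component.
; Each tick it reads the widget's Selected flag; once that is true, it destroys itself and spawns BP_MenuSand at the same transform.
; This polling swaps menu screens by replacing whole actors rather than changing widget content.
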(event `self.ReceiveBeginPlay`)

(event `self.ReceiveTick`
  (params (DeltaSeconds :type "Float (single-precision)"))
  (bind _askiosk_main (cast `/Game/BP/SubwayWidget/Kiosk_Main` (`WidgetComponent.GetWidget` (`self.Widget`))))
  (if (`/Game/BP/SubwayWidget/Kiosk_Main.Selected` _askiosk_main)
    (`self.K2_DestroyActor`)
    (`|SpawnActorFromClass` "/Game/BP/SubwayWidget/BP_MenuSand.BP_MenuSand_C" (`self.GetTransform`) "Undefined" "MultiplyWithRoot" null null)))

(fn `UserConstructionScript`)