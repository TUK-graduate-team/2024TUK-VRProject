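; BP_MenuSelectPay is the payment method selection screen of a Subway kiosk menu, an actor hosting a Kiosk_Selectpay widget.
; Tick polls the widget's flags and moves between screens by destroying this actor and spawning the next at the same transform.
; Pre returns to BP_MenuSand, while Selected uses JudgePay to open BP_MenuPayCredit for credit card or BP_MenuPayNaver for Naver Pay.
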(event `self.ReceiveBeginPlay`)

(event `self.ReceiveTick`
  (params (DeltaSeconds :type "Float (single-precision)"))
  (bind _returnvalue (`WidgetComponent.GetWidget` (`self.Widget`)))
  (bind _askiosk_selectpay (cast `/Game/BP/SubwayWidget/Kiosk_Selectpay` _returnvalue))
  (if (`/Game/BP/SubwayWidget/Kiosk_Selectpay.Pre` _askiosk_selectpay)
    (`self.K2_DestroyActor`)
    (`|SpawnActorFromClass` "/Game/BP/SubwayWidget/BP_MenuSand.BP_MenuSand_C" (`self.GetTransform`) "Undefined" "MultiplyWithRoot" null null)
    (else
      (bind _askiosk_selectpay_2 (cast `/Game/BP/SubwayWidget/Kiosk_Selectpay` _returnvalue))
      (if (`/Game/BP/SubwayWidget/Kiosk_Selectpay.Selected` _askiosk_selectpay_2)
        ;[1 1 1] 1은 신용카드, 2는 네이버페이
        (bind _askiosk_selectpay_3 (cast `/Game/BP/SubwayWidget/Kiosk_Selectpay` (`WidgetComponent.GetWidget` (`self.Widget`))))
        (`/Engine/EditorBlueprintResources/StandardMacros.CompareInt` (`/Game/BP/SubwayWidget/Kiosk_Selectpay.JudgePay` _askiosk_selectpay_3) 2
          (:`==`
            (`self.K2_DestroyActor`)
            (`|SpawnActorFromClass` "/Game/BP/SubwayWidget/BP_MenuPayNaver.BP_MenuPayNaver_C" (`self.GetTransform`) "Undefined" "MultiplyWithRoot" null null))
          (:`<`
            (`self.K2_DestroyActor`)
            (`|SpawnActorFromClass` "/Game/BP/SubwayWidget/BP_MenuPayCredit.BP_MenuPayCredit_C" (`self.GetTransform`) "Undefined" "MultiplyWithRoot" null null)))))))

(fn `UserConstructionScript`)