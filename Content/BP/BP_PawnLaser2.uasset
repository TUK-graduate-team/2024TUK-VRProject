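; BP_PawnLaser2 is a VR pawn that spawns a pair of BP_Hand actors and forwards pinch input to them.
; On BeginPlay it sets a floor-level tracking origin, then spawns left and right hands owned by the pawn and attaches each to itself with snap rules.
; Left and right middle-finger pinch input actions call Press and Release on the matching hand, leaving the interaction behavior to BP_Hand.
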(event `self.ReceiveBeginPlay`
  (bind _returnvalue (`KismetMathLibrary.MakeTransform` (0.0 0.0 0.0)))
  (`|ExecutionSequence`
    (:`then_0`
      (`HeadMountedDisplayFunctionLibrary.SetTrackingOrigin` "Floor"))
    (:`then_1`
      (`|ExecutionSequence`
        (:`then_0`
          (bind _returnvalue_2 (`|SpawnActorFromClass` "/Game/BP/BP_Hand.BP_Hand_C" _returnvalue "AlwaysSpawn" "MultiplyWithRoot" self "Left" null))
          (bind _output_get (set `self.Left` _returnvalue_2))
          (`self.K2_AttachToActor` _output_get self "None" "SnapToTarget" "SnapToTarget" "SnapToTarget" true))
        (:`then_1`
          (bind _returnvalue_3 (`|SpawnActorFromClass` "/Game/BP/BP_Hand.BP_Hand_C" _returnvalue "AlwaysSpawn" "MultiplyWithRoot" self "Right" null))
          (bind _output_get_2 (set `self.Right` _returnvalue_3))
          (`self.K2_AttachToActor` _output_get_2 self "None" "SnapToTarget" "SnapToTarget" "SnapToTarget" true))))))

(event `InputAction|LeftMiddlePinch`
  (params (Key :type "Key Structure"))
  (bind _left (`self.Left`))
  (:`Pressed`
    (`/Game/BP/BP_Hand.Press` _left))
  (:`Released`
    (`/Game/BP/BP_Hand.Release` _left)))

(event `InputAction|RightMiddlePinch`
  (params (Key :type "Key Structure"))
  (bind _right (`self.Right`))
  (:`Pressed`
    (`/Game/BP/BP_Hand.Press` _right))
  (:`Released`
    (`/Game/BP/BP_Hand.Release` _right)))

(fn `UserConstructionScript`)