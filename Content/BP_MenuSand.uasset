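; BP_MenuSand is a kiosk menu screen actor that hosts the Kiosk_sand widget through its Widget component.
; Each tick it polls the widget's Selected flag, then uses its Next flag to choose the following screen.
; It destroys itself and spawns BP_MenuSelectPay when Next is set, otherwise BP_MenuMain, at the same transform, so navigation works by swapping whole actors.
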(event `self.ReceiveBeginPlay`)

(event `self.ReceiveTick`
  (params (DeltaSeconds :type "Float (single-precision)"))
  (bind _returnvalue (`WidgetComponent.GetWidget` (`self.Widget`)))
  (bind _askiosk_sand (cast `/Game/Kiosk_sand` _returnvalue))
  (if (`/Game/Kiosk_sand.Selected` _askiosk_sand)
    (bind _askiosk_sand_2 (cast `/Game/Kiosk_sand` _returnvalue))
    (if (`/Game/Kiosk_sand.Next` _askiosk_sand_2)
      (`self.K2_DestroyActor`)
      (`|SpawnActorFromClass` "/Game/BP_MenuSelectPay.BP_MenuSelectPay_C" (`self.GetTransform`) "Undefined" "MultiplyWithRoot" null null)
      (else
        (`self.K2_DestroyActor`)
        (`|SpawnActorFromClass` "/Game/BP_MenuMain.BP_MenuMain_C" (`self.GetTransform`) "Undefined" "MultiplyWithRoot" null null)))))

(fn `UserConstructionScript`)